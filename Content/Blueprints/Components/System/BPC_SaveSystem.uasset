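; Actor component that makes its owner saveable, persisting location, rotation and logic state under a GUID SaveID.
; On BeginPlay a valid ID registers it with the GameInstance's save system, then it pulls the save game and restores each stored value.
; SaveData writes values into ID-keyed maps in the passed save object.
; Owner interface messages supply and apply the data, with a savable flag per category.
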(event Custom|GenerateID
  (if (not (Guid|IsValidGuid (Variables|Default|GetSaveID)))
    (Variables|Default|SetSaveID (Guid|NewGuid))))

(event EventBeginPlay
  (if (Guid|IsValidGuid (Variables|Default|GetSaveID))
    (bind _success (Class|BPISaveLoadGame|SendSaveableObject(Message) (Game|GetGameInstance) self))
    (bind _output_get (Variables|Default|SetInSavedSystem _success))
    (if _output_get
      (CallFunction|GetLoadData))))

(fn GetLoadData
  (Variables|Default|GetInSavedSystem
    (:then
      (bind _returnvalue (Class|BPISaveLoadGame|GetSaveGame(Message) (Game|GetGameInstance)))
      (Utilities|IsValid _returnvalue
        (:Is%20Valid
          (LocalVariables|SetL_SaveGame _returnvalue)
          (LoadData|LoadLocationData (LocalVariables|GetL_SaveGame))
          (LoadData|LoadRotationData (LocalVariables|GetL_SaveGame))
          (LoadData|LoadLogicData (LocalVariables|GetL_SaveGame))
          (return))
        (:Is%20Not%20Valid
          (return))))
    (:else)))

(fn SaveLocationData
  (params (InSaveData :type BP%20Save%20Game%20Object%20Reference))
  (bind (_issavable _returnlocation) (Class|BPIBPISaveable|GetLocationSaveData(Message) (Components|GetOwner)))
  (if _issavable
    (Utilities|Map|Add (Variables|/Game/Blueprints/Core/BP_SaveGame.BP_SaveGame_C|GetObjectsLocationData InSaveData) (Variables|Default|GetSaveID) _returnlocation)
    (return)
    (else
      (return))))

(fn LoadLocationData
  (params (InSaveGame :type BP%20Save%20Game%20Object%20Reference%20%28by%20ref%29))
  (bind _objectslocationdata (Variables|/Game/Blueprints/Core/BP_SaveGame.BP_SaveGame_C|GetObjectsLocationData InSaveGame))
  (bind _saveid (Variables|Default|GetSaveID))
  (bind (_value _returnvalue) (Utilities|Map|Find _objectslocationdata _saveid))
  (if _returnvalue
    (Class|BPIBPISaveable|SetLocationLoadData(Message) (Components|GetOwner) _value)
    (return)
    (else
      (return))))

(fn SaveRotationData
  (params (InSaveData :type BP%20Save%20Game%20Object%20Reference))
  (bind (_issavable _returnrotation) (Class|BPIBPISaveable|GetRotationSaveData(Message) (Components|GetOwner)))
  (if _issavable
    (Utilities|Map|Add (Variables|/Game/Blueprints/Core/BP_SaveGame.BP_SaveGame_C|GetObjectsRotationData InSaveData) (Variables|Default|GetSaveID) _returnrotation)
    (return)
    (else
      (return))))

(fn LoadRotationData
  (params (InSaveData :type BP%20Save%20Game%20Object%20Reference%20%28by%20ref%29))
  (bind _objectsrotationdata (Variables|/Game/Blueprints/Core/BP_SaveGame.BP_SaveGame_C|GetObjectsRotationData InSaveData))
  (bind _saveid (Variables|Default|GetSaveID))
  (bind (_value _returnvalue) (Utilities|Map|Find _objectsrotationdata _saveid))
  (if _returnvalue
    (Class|BPIBPISaveable|SetRotationLoadData(Message) (Components|GetOwner) _value)
    (return)
    (else
      (return))))

(fn SaveLogicData
  (params (InSaveData :type BP%20Save%20Game%20Object%20Reference))
  (bind (_issavable _returnrotation) (Class|BPIBPISaveable|GetLogicSaveData(Message) (Components|GetOwner)))
  (if _issavable
    (Utilities|Map|Add (Variables|/Game/Blueprints/Core/BP_SaveGame.BP_SaveGame_C|GetObjectsLogicData InSaveData) (Variables|Default|GetSaveID) _returnrotation)
    (return)
    (else
      (return))))

(fn LoadLogicData
  (params (InSaveData :type BP%20Save%20Game%20Object%20Reference%20%28by%20ref%29))
  (bind _objectslogicdata (Variables|/Game/Blueprints/Core/BP_SaveGame.BP_SaveGame_C|GetObjectsLogicData InSaveData))
  (bind _saveid (Variables|Default|GetSaveID))
  (bind (_value _returnvalue) (Utilities|Map|Find _objectslogicdata _saveid))
  (if _returnvalue
    (Class|BPIBPISaveable|SetLogicLoadData(Message) (Components|GetOwner) _value)
    (return)
    (else
      (return))))

(fn PlayerLoadData
  (params (InLoadData :type BP%20Save%20Game%20Object%20Reference%20%28by%20ref%29)))

(fn SaveData
  (params (InSaveData :type BP%20Save%20Game%20Object%20Reference%20%28by%20ref%29))
  (Variables|Default|GetInSavedSystem
    (:then
      (SaveData|SaveLocationData InSaveData)
      (SaveData|SaveRotationData InSaveData)
      (SaveData|SaveLogicData InSaveData)
      (return true))
    (:else
      (return false))))