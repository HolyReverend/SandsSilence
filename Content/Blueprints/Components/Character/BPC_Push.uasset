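; Character component that lets its owner push pushable actors, talking to the character through interface messages.
; BeginPushing picks the nearest attach point, validates ground, space, slope and obstacles, then slides the capsule there and attaches the object to the character.
; A looping timer traces along the input direction to switch movement modes when free or blocked, and ends pushing when an obstacle separates character and object.
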(event Custom|AttachToPushableObject
  (params (InAttachLocation :type Vector%20%28by%20ref%29) (InAttachRotation :type Rotator%20%28by%20ref%29) (InAttachTimeDuration :type Float%20%28double-precision%29%20%28by%20ref%29))
  (Class|BPIPlayerCharacter|SwitchCharacterMovementMode(Message) (Components|GetOwner) "NewEnumerator8")
  (bind _returnvalue (Class|BPIPlayerCharacter|GetCharacterCapsuleComponent(Message) (Components|GetOwner)))
  (Components|MoveComponentTo _returnvalue InAttachLocation InAttachRotation true true InAttachTimeDuration true)
  (CallFunction|StartPushing))

(event EventEndPlay
  (params (EndPlayReason :type EEndPlayReason%20Enum :default "Destroyed"))
  (|CallParentFunction EndPlayReason)
  (System|ClearUp))

(fn FindNearestAttachPointIndex
  (params (InPushableActor :type Actor%20Object%20Reference) (InPushAttachPoints :type Array%20of%20Transforms))
  (if (Utilities|Array|IsNotEmpty InPushAttachPoints)
    (if (> (Utilities|Array|Length InPushAttachPoints) 1)
      (for (_array_element _array_index) InPushAttachPoints
        (LocalVariables|SetL_CurrentAttachPointIndex _array_index)
        (LocalVariables|SetL_CurrentAttachPointDistanceSq (Class|KismetMathLibrary|DistanceSquared2D (Math|Conversions|ToVector2D(Vector) (Math|Transform|TransformLocation (Transformation|GetActorTransform InPushableActor) (.location _array_element))) (Math|Conversions|ToVector2D(Vector) (Transformation|GetActorLocation (Components|GetOwner)))))
        (bind _returnvalue (Class|BPIPlayerCharacter|GetCharacterHalfHeight(Message) (Components|GetOwner)))
        (if (> (Math|Float|Square _returnvalue) (LocalVariables|GetL_CurrentAttachPointDistanceSq))
          (if (or (< (LocalVariables|GetL_CurrentAttachPointDistanceSq) (LocalVariables|GetL_NearestAttachPointDistanceSq)) (< (LocalVariables|GetL_NearestAttachPointIndex) 0))
            (LocalVariables|SetL_NearestAttachPointIndex (LocalVariables|GetL_CurrentAttachPointIndex))
            (LocalVariables|SetL_NearestAttachPointDistanceSq (LocalVariables|GetL_CurrentAttachPointDistanceSq)))))
      (return (LocalVariables|GetL_NearestAttachPointIndex))
      (else
        (return 1)))
    (else
      (return -1))))

(fn StartPushing
  (Variables|Default|GetCurrentPushingActor
    (:then
      (bind _returnvalue (Transformation|AttachActorToActor (Variables|Default|GetCurrentPushingActor) (Components|GetOwner) "None" "KeepWorld" "KeepWorld" "KeepWorld" false))
      (if _returnvalue
        (Class|BPIPlayerCharacter|SendSpeedMult(Message) (Components|GetOwner) (Default|GetMovableSpeedMult (Variables|Default|GetCurrentPushingActor)))
        (Class|BPIPlayerCharacter|SwitchCharacterMovementMode(Message) (Components|GetOwner) "NewEnumerator7")
        (bind _returnvalue_2 (Utilities|Time|SetTimerbyEvent (EventDispatchers|CreateEvent :!event PushStateUpdate) 0.1 true))
        (Variables|Default|SetPushStateUpdateHandler _returnvalue_2)
        (return)
        (else
          (Utilities|PushFailInfo "Не удалось приатачить пушиемого актора к персонажу")
          (return))))
    (:else
      (return))))

(fn CheckPushPath
  (bind (_outobjecttypes _outactorstoignore _outdrawdebugtype) (CallFunction|GetPushTraceSettings))
  (bind _returnvalue (Components|GetOwner))
  (bind (_outobjecttypes_2 _outactorstoignore_2 _outdrawdebugtype_2) (CallFunction|GetPushTraceSettings))
  (bind _currentpushingactor (Variables|Default|GetCurrentPushingActor))
  (bind _pushablemesh (Variables|/Game/Blueprints/Logic/Pushable/BP_PushableBase.BP_PushableBase_C|GetPushableMesh _currentpushingactor))
  (bind _max (Components|StaticMesh|GetLocalBounds _pushablemesh))
  (bind _returnvalue_2 (Class|BPIPlayerCharacter|GetMovementAxisValue(Message) (Components|GetOwner)))
  (if (Class|KismetMathLibrary|NotEqualExactlyVector2DVector2D _returnvalue_2)
    (bind _outhit (Class|KismetSystemLibrary|BoxTraceSingleforObjects (+ (Transformation|GetWorldLocation (Variables|/Game/Blueprints/Logic/Pushable/BP_PushableBase.BP_PushableBase_C|GetPushableMesh (Variables|Default|GetCurrentPushingActor))) (* (+ (* (Transformation|GetActorForwardVector _returnvalue) (.Y (Math|Vector2D|BreakVector2D _returnvalue_2))) (* (Transformation|GetActorRightVector _returnvalue) (.X (Math|Vector2D|BreakVector2D _returnvalue_2)))) (.X (Math|Vector|BreakVector _max)))) (+ (Transformation|GetWorldLocation (Variables|/Game/Blueprints/Logic/Pushable/BP_PushableBase.BP_PushableBase_C|GetPushableMesh (Variables|Default|GetCurrentPushingActor))) (* (+ (* (Transformation|GetActorForwardVector _returnvalue) (.Y (Math|Vector2D|BreakVector2D _returnvalue_2))) (* (Transformation|GetActorRightVector _returnvalue) (.X (Math|Vector2D|BreakVector2D _returnvalue_2)))) (.X (Math|Vector|BreakVector _max)))) (* _max (Transformation|GetWorldScale _pushablemesh)) (Transformation|GetWorldRotation _pushablemesh) _outobjecttypes_2 false _outactorstoignore_2 _outdrawdebugtype_2 true "(R=0.173198,G=0.000000,B=1.000000,A=1.000000)" "(R=1.000000,G=0.012178,B=0.000000,A=1.000000)" 0.1))
    (if (or (not (.bBlockingHit (Collision|BreakHitResult _outhit))) (not (.bInitialOverlap (Collision|BreakHitResult _outhit))))
      (bind _outhit_2 (Collision|LineTraceForObjects (Transformation|GetActorLocation (Components|GetOwner)) (Transformation|GetWorldLocation (Variables|/Game/Blueprints/Logic/Pushable/BP_PushableBase.BP_PushableBase_C|GetPushableMesh (Variables|Default|GetCurrentPushingActor))) _outobjecttypes false _outactorstoignore _outdrawdebugtype true "(R=0.000000,G=0.051395,B=1.000000,A=1.000000)" "(R=1.000000,G=0.077227,B=0.000000,A=1.000000)" 0.1))
      (if (not (or (.bBlockingHit (Collision|BreakHitResult _outhit_2)) (.bInitialOverlap (Collision|BreakHitResult _outhit_2))))
        (return "NewEnumerator0")
        (else
          (return "NewEnumerator2")))
      (else
        (return "NewEnumerator1")))
    (else
      (return "NewEnumerator1"))))

(fn ClearUp
  (Utilities|Array|Clear (Variables|Default|GetActorsToIgnore))
  (Variables|Default|SetCurrentPushingActor 0)
  (Variables|Default|SetPushStateUpdateHandler "")
  (return))

(fn GetPushTraceSettings
  (return (Utilities|Array|MakeArray "ObjectTypeQuery1" "ObjectTypeQuery2") (Variables|Default|GetActorsToIgnore) (select (Variables|Debug|GetDebug_Status) "ForDuration" "None")))

(fn PushStateUpdate
  (bind _returnvalue (Components|GetOwner))
  (switch Utilities|FlowControl|Switch|SwitchonE_PushableStatus (CallFunction|CheckPushPath)
    (:NewEnumerator0
      (Class|BPIPlayerCharacter|SwitchCharacterMovementMode(Message) _returnvalue "NewEnumerator7")
      (return))
    (:NewEnumerator1
      (Class|BPIPlayerCharacter|SwitchCharacterMovementMode(Message) _returnvalue "NewEnumerator8")
      (return))
    (:NewEnumerator2
      (CallFunction|EndPushing (Variables|Default|GetCurrentPushingActor))
      (return))))

(fn BeginPushing
  (params (InPushableActor :type BP%20Pushable%20Base%20Object%20Reference%20%28by%20ref%29) (InPushAttachPoints :type Array%20of%20Transforms) (InAttachTimeDuration :type Float%20%28double-precision%29%20%28by%20ref%29))
  (bind (_outobjecttypes _outactorstoignore _outdrawdebugtype) (CallFunction|GetPushTraceSettings))
  (bind _returnvalue (Transformation|GetActorTransform InPushableActor))
  (bind _nearestattachpointindex (CallFunction|FindNearestAttachPointIndex InPushableActor InPushAttachPoints))
  (bind _output (Utilities|Array|Get(acopy) InPushAttachPoints _nearestattachpointindex))
  (bind _returnvalue_2 (Math|Transform|ComposeTransforms _output _returnvalue))
  (Utilities|Array|Clear (Variables|Default|GetActorsToIgnore))
  (LocalVariables|GetInPushableActor
    (:then
      (bind _isvalid (Class|BPIPlayerCharacter|CheckIsCharacteronGround(Message) (Components|GetOwner)))
      (if _isvalid
        (if (>= _nearestattachpointindex 0)
          (bind _returnvalue_3 (Class|BPIPlayerCharacter|GetCharacterHalfHeight(Message) (Components|GetOwner)))
          (bind _output_get (LocalVariables|SetL_CharacterHalfHeight _returnvalue_3))
          (LocalVariables|SetL_TargetAttachPoint (Math|Transform|MakeTransform (+ (Math|Vector|MakeVector 0.0 0.0 _output_get) (.location _returnvalue_2)) (.rotation _returnvalue_2) (.scale _returnvalue_2)))
          (Utilities|Array|AddUnique (Variables|Default|GetActorsToIgnore) InPushableActor)
          (bind _returnvalue_4 (Class|BPIPlayerCharacter|GetCharacterRaduis(Message) (Components|GetOwner)))
          ;[0.15 0.15 0.15 0.5] Проверяем может ли персонаж вместиться в точку прикрепления к объекту
          (bind _outhit (Collision|CapsuleTraceByChannel (+ (.location (LocalVariables|GetL_TargetAttachPoint)) "0.000000,0.000000,70.000000") (+ (.location (LocalVariables|GetL_TargetAttachPoint)) "0.000000,0.000000,-100.000000") _returnvalue_4 (LocalVariables|GetL_CharacterHalfHeight) "TraceTypeQuery1" false (Variables|Default|GetActorsToIgnore) (select (Variables|Debug|GetDebug_Status) "ForDuration" "None") true "(R=0.164130,G=0.000000,B=1.000000,A=1.000000)" "(R=1.000000,G=0.103472,B=0.000383,A=1.000000)" 2.0))
          (if (not (.bInitialOverlap (Collision|BreakHitResult _outhit)))
            (bind _returnvalue_5 (Class|BPIPlayerCharacter|GetCharacterWalkableFloorZ(Message) (Components|GetOwner)))
            (if (< _returnvalue_5 (.Z (Math|Vector|BreakVector (.ImpactNormal (Collision|BreakHitResult _outhit)))))
              ;[0.15 0.15 0.15 0.5] Проверка есть ли между персонажем и объектом препятствие
              (bind _returnvalue_6 (Collision|LineTraceForObjects (Transformation|GetActorLocation InPushableActor) (.location (LocalVariables|GetL_TargetAttachPoint)) _outobjecttypes false _outactorstoignore _outdrawdebugtype true "(R=0.030007,G=0.000000,B=1.000000,A=1.000000)" "(R=1.000000,G=0.110468,B=0.000000,A=1.000000)" 2.0))
              (if (not _returnvalue_6)
                (Class|BPIPlayerCharacter|SendResetSpeedandJump(Message) (Components|GetOwner) false)
                (Variables|Default|SetCurrentPushingActor InPushableActor)
                (CallFunction|AttachtoPushableObject (.Location (Math|Transform|BreakTransform (LocalVariables|GetL_TargetAttachPoint))) (.Rotation (Math|Transform|BreakTransform (LocalVariables|GetL_TargetAttachPoint))) InAttachTimeDuration)
                (return true)
                (else
                  (Utilities|PushFailInfo "Между персонажем и объектом препятствие")
                  (return false)))
              (else
                (Utilities|PushFailInfo "Слишком крутой склон")
                (return false)))
            (else
              (Utilities|PushFailInfo "Нет места для персонажа")
              (return false)))
          (else
            (Utilities|PushFailInfo "Не найдено точек крепления")
            (return false)))
        (else
          (Utilities|PushFailInfo "Персонаж не на земле")
          (return false))))
    (:else
      (return false))))

(fn CheckCharactaerIsPushing
  (Variables|Default|GetCurrentPushingActor
    (:then
      (return true))
    (:else
      (return false))))

(fn EndPushing
  (params (InPushableActor :type BP%20Pushable%20Base%20Object%20Reference%20%28by%20ref%29))
  (if (and (== InPushableActor (Variables|Default|GetCurrentPushingActor)) (Utilities|IsValid (Variables|Default|GetCurrentPushingActor)))
    (Class|BPIPlayerCharacter|SendResetSpeedandJump(Message) (Components|GetOwner) false)
    (Transformation|DetachFromActor (Variables|Default|GetCurrentPushingActor) "KeepWorld" "KeepWorld" "KeepWorld")
    (Utilities|Time|ClearandInvalidateTimerbyHandle (Variables|Default|GetPushStateUpdateHandler))
    (Class|BPIPlayerCharacter|SendSpeedMult(Message) (Components|GetOwner) 1.0)
    (Class|BPIPlayerCharacter|SwitchCharacterMovementMode(Message) (Components|GetOwner) "NewEnumerator1")
    (Variables|Default|SetCurrentPushingActor 0)
    (return true)
    (else
      (return false))))