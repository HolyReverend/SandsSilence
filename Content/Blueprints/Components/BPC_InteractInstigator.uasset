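; Actor component that lets its owner act as an interaction instigator, tracking interactable actors and triggering their use.
; Add and remove functions maintain the list, accepting only actors that implement BPI_Interactable.
; On use, it sends StartInteractMessage to the candidate nearest the owner and returns the result.
; Candidates are narrowed to actors carrying their own BPC_InteractInstigator when any exist, otherwise the whole list is used.
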(fn InstigatersPrioritization
  (for _array_element (Variables|Default|GetInteractableActors)
    (if (Utilities|IsValid (Actor|GetComponentbyClass _array_element "BPC_InteractInstigator_C"))
      (Utilities|Array|AddUnique (LocalVariables|GetInstigaters) _array_element)))
  (if (Utilities|Array|IsNotEmpty (LocalVariables|GetInstigaters))
    (return (LocalVariables|GetInstigaters))
    (else
      (return (Variables|Default|GetInteractableActors)))))

(fn ActionInteractableUse
  (if (Utilities|Array|IsNotEmpty (Variables|Default|GetInteractableActors))
    (bind _success (Class|BPIInteractable|StartInteract(Message) (.ReturnValue (Actor|FindNearestActor (Transformation|GetActorLocation (Components|GetOwner)) (CallFunction|InstigatersPrioritization))) (Components|GetOwner) true))
    (return _success)
    (else
      (return false))))

(fn AddInteractableActor
  (params (InInteractableActor :type Actor%20Object%20Reference%20%28by%20ref%29))
  (if (Utilities|DoesObjectImplementInterface InInteractableActor "/Game/Blueprints/Interfaces/BPI_Interactable.BPI_Interactable_C")
    (Utilities|Array|AddUnique (Variables|Default|GetInteractableActors) InInteractableActor)
    (return true (Components|GetOwner))
    (else
      (return false (Components|GetOwner)))))

(fn CheckImplementInteract
  (return true))

(fn RemoveInteractableActor
  (params (InInteractableActor :type Actor%20Object%20Reference%20%28by%20ref%29))
  (Utilities|Array|RemoveItem (Variables|Default|GetInteractableActors) InInteractableActor)
  (return true (Components|GetOwner)))