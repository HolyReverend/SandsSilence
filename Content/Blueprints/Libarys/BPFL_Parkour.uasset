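; Blueprint function library of pure helpers for the parkour system.
; Two functions turn a rotation 180 degrees around yaw, one of them deriving the yaw from a surface normal.
; The Select functions switch on Parkour gameplay tags for climb style, direction or state and return the matching caller-supplied value.
; Direction selection covers eight directions, with a float variant and a hop-action tag variant.
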(fn NormalReverseRotationZ
  (params (InNormal :type Vector%20%28by%20ref%29))
  ;[0.15 0.15 0.15 0.5] Развернуть на 180 градусов нормаль по Z (Yaw)
  (return (Math|Rotator|MakeRotator 0.0 0.0 (.yaw (Math|Rotator|Delta(Rotator) (Math|Rotator|MakeRotfromX InNormal) "0.000000,180.000000,0.000000")))))

(fn ReverseRotationZ
  (params (InRotation :type Rotator%20%28by%20ref%29))
  ;[0.15 0.15 0.15 0.5] Развернуть на 180 градусов по оси Z
  (return (Math|Rotator|Delta(Rotator) InRotation "0.000000,180.000000,0.000000")))

(fn SelectClimbStyleFloat
  (params (InBraced :type Float%20%28double-precision%29%20%28by%20ref%29) (InFreeHang :type Float%20%28double-precision%29%20%28by%20ref%29) (InClimbStyle :type Gameplay%20Tag%20Structure%20%28by%20ref%29))
  ;[0.15 0.15 0.15 0.5] Выбор значения в соответствии с Climb-стилем
  (|SwitchGameplayTag InClimbStyle
    (:Parkour.ClimbStyle.Braced
      (return InBraced))
    (:Parkour.ClimbStyle.FreeHang
      (return InFreeHang))))

(fn SelectDirectionFloat
  (params (InForward :type Float%20%28double-precision%29%20%28by%20ref%29) (InBackward :type Float%20%28double-precision%29%20%28by%20ref%29) (InLeft :type Float%20%28double-precision%29%20%28by%20ref%29) (InRight :type Float%20%28double-precision%29%20%28by%20ref%29) (InForwardLeft :type Float%20%28double-precision%29%20%28by%20ref%29) (InForwardRight :type Float%20%28double-precision%29%20%28by%20ref%29) (InBackwardLeft :type Float%20%28double-precision%29%20%28by%20ref%29) (InBackwardRight :type Float%20%28double-precision%29%20%28by%20ref%29) (InDirection :type Gameplay%20Tag%20Structure%20%28by%20ref%29))
  ;[0.15 0.15 0.15 0.5] Выбор значения в соответствии с Direction
  (|SwitchGameplayTag InDirection
    (:Parkour.Direction.Forward
      (return InForward))
    (:Parkour.Direction.Backward
      (return InBackward))
    (:Parkour.Direction.Left
      (return InLeft))
    (:Parkour.Direction.Right
      (return InRight))
    (:Parkour.Direction.ForwardLeft
      (return InForwardLeft))
    (:Parkour.Direction.ForwardRight
      (return InForwardRight))
    (:Parkour.Direction.BackwardLeft
      (return InBackwardLeft))
    (:Parkour.Direction.BackwardRight
      (return InBackwardRight))))

(fn SelectParkourStateFloat
  (params (InNotBusy :type Float%20%28double-precision%29%20%28by%20ref%29) (InVault :type Float%20%28double-precision%29%20%28by%20ref%29) (InMantle :type Float%20%28double-precision%29%20%28by%20ref%29) (InClimb :type Float%20%28double-precision%29%20%28by%20ref%29) (InParkourState :type Gameplay%20Tag%20Structure%20%28by%20ref%29))
  ;[0.15 0.15 0.15 0.5] Выбрать значение для Parkour-состояния
  (|SwitchGameplayTag InParkourState
    (:Parkour.State.NotBusy
      (return InNotBusy))
    (:Parkour.State.Vault
      (return InVault))
    (:Parkour.State.Mantle
      (return InMantle))
    (:Parkour.State.Climb
      (return InClimb))))

(fn SelectDirectionHopAction
  (params (InForward :type Gameplay%20Tag%20Structure%20%28by%20ref%29) (InBackward :type Gameplay%20Tag%20Structure%20%28by%20ref%29) (InLeft :type Gameplay%20Tag%20Structure%20%28by%20ref%29) (InRight :type Gameplay%20Tag%20Structure%20%28by%20ref%29) (InForwardLeft :type Gameplay%20Tag%20Structure%20%28by%20ref%29) (InForwardRight :type Gameplay%20Tag%20Structure%20%28by%20ref%29) (InBackwardLeft :type Gameplay%20Tag%20Structure%20%28by%20ref%29) (InBackwardRight :type Gameplay%20Tag%20Structure%20%28by%20ref%29) (InDirection :type Gameplay%20Tag%20Structure%20%28by%20ref%29))
  ;[0.15 0.15 0.15 0.5] Выбор тага в соответствии с Direction
  (|SwitchGameplayTag InDirection
    (:Parkour.Direction.Forward
      (return InForward))
    (:Parkour.Direction.Backward
      (return InBackward))
    (:Parkour.Direction.Left
      (return InLeft))
    (:Parkour.Direction.Right
      (return InRight))
    (:Parkour.Direction.ForwardLeft
      (return InForwardLeft))
    (:Parkour.Direction.ForwardRight
      (return InForwardRight))
    (:Parkour.Direction.BackwardLeft
      (return InBackwardLeft))
    (:Parkour.Direction.BackwardRight
      (return InBackwardRight))))