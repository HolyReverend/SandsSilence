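; General-purpose Blueprint function library of small gameplay, debug and math helpers.
; Player helpers return the pawn controlled by player controller 0 or check whether a given actor is that pawn.
; A debug helper prints a colored dashed separator on screen with a given duration and key, without logging.
; The float AlwaysNegative forces a negative sign through Abs, while the integer version only flips the sign, so negative inputs become positive.
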(fn CheckIsPlayer
  (params (InActor :type Actor%20Object%20Reference%20%28by%20ref%29))
  ;[0.15 0.15 0.15 0.5] Проверка является ли Актор игровым персонажем
  (return (== InActor (Pawn|GetControlledPawn (Game|GetPlayerController 0)))))

(fn PrintSeparator
  (params (InTimeDuration :type Float%20%28single-precision%29%20%28by%20ref%29) (InKey :type Name%20%28by%20ref%29))
  ;[0.15 0.15 0.15 0.5] Напечатать на экран разделитель
  (Development|PrintText 0 (Utilities|Text|FormatText "--------------------------------") true false "(R=0.896269,G=0.032944,B=0.000000,A=1.000000)" InTimeDuration InKey)
  (return))

(fn GetActualPlayer
  (return (Pawn|GetControlledPawn (Game|GetPlayerController 0))))

(fn AlwaysNegative(Float)
  (params (InValue :type Float%20%28double-precision%29))
  (return (* (Math|Float|Absolute(Float) InValue) -1.0)))

(fn AlwaysNegative(Integer)
  (params (InValue :type Integer))
  (return (* InValue -1)))