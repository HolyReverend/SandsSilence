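; Base GameState Blueprint that holds temporary save data for objects and the player.
; Object data is kept in a map keyed by GUID, while player data is a single stored value.
; Simple getters return both stores, and setters add an object entry or replace the player data, always returning true.
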(fn ConstructionScript)

(fn GetTempObjectsData
  (return (Variables|SaveLoadSystem|GetTempObjectsData)))

(fn GetTempPlayerData
  (return (Variables|SaveLoadSystem|GetTempPlayerData)))

(fn SetTempObjectData
  (params (InGuid :type Guid%20Structure) (InSaveData :type ST%20Object%20Save%20Data%20Structure))
  (Utilities|Map|Add (Variables|SaveLoadSystem|GetTempObjectsData) InGuid InSaveData)
  (return true))

(fn SetTempPlayerData
  (params (InSaveData :type ST%20Player%20Save%20Data%20Structure%20%28by%20ref%29))
  (Variables|SaveLoadSystem|SetTempPlayerData InSaveData)
  (return true))