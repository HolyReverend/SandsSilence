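; Game state Blueprint that hands random static meshes to requesting actors through the BPI_Actor interface.
; On BeginPlay it async-loads DA_MeshArray and caches its mesh list, queuing earlier requests to repeat once loaded.
; Each request uses an already loaded soft reference directly or async-loads one, with separate random picks for check and use.
; A single SourceRequest variable holds the pending requester, and EndPlay clears cached references.
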(event EventBeginPlay
  (bind _object (Utilities|AsyncLoadAsset "/Game/Blueprints/TestActor/DA_MeshArray.DA_MeshArray")
    (:Completed
      (bind _asbpi_mesh_array (Utilities|Casting|CastToBPI_MeshArray _object))
      (bind _output_get (Variables|Default|SetAs%20BPI%20Mesh%20Array _asbpi_mesh_array))
      (bind _mesharray (Default|GetMeshArray _output_get))
      (Variables|Default|SetMeshArray _mesharray)
      (Variables|Default|SetisConfigLoaded true)
      (for _array_element (Variables|Default|GetRequeRequest)
        (Default|RepeatRequest _array_element))
      (Utilities|Array|Clear (Variables|Default|GetRequeRequest)))))

(event EventEndPlay
  (params (EndPlayReason :type EEndPlayReason%20Enum :default "Destroyed"))
  (CallFunction|ClearUP))

(event EventRequestRandomMesh
  (params (SourceRequest :type Object%20Object%20Reference))
  (bind (_success _randommesh) (CallFunction|GetRandomMesh))
  (bind _asbpi_actor (Utilities|Casting|CastToBPI_Actor SourceRequest))
  (Variables|Default|SetSourceRequest _asbpi_actor)
  (if (Variables|Default|GetisConfigLoaded)
    (if _success
      (Default|SetRandomMesh (Variables|Default|GetSourceRequest) (Utilities|ResolveSoftReference _randommesh))
      (else
        (bind _object (Utilities|AsyncLoadAsset _randommesh)
          (:then
            (bind _asstatic_mesh (Utilities|Casting|CastToStaticMesh _object))
            (Default|SetRandomMesh (Variables|Default|GetSourceRequest) _asstatic_mesh)))))
    (Variables|Default|SetSourceRequest 0)
    (else
      (Utilities|Array|AddUnique (Variables|Default|GetRequeRequest) (Variables|Default|GetSourceRequest)))))

(fn ConstructionScript)

(fn ClearUP
  (Variables|Default|SetAs%20BPI%20Mesh%20Array 0)
  (Utilities|Array|Clear (Variables|Default|GetMeshArray))
  (Utilities|Array|Clear (Variables|Default|GetRequeRequest))
  (Variables|Default|SetSourceRequest 0))

(fn GetRandomMesh
  (bind _output_get (LocalVariables|SetL_RandomMesh (.OutItem (Utilities|Array|Random (Variables|Default|GetMeshArray)))))
  (return (Utilities|IsValidSoftObjectReference _output_get) (LocalVariables|GetL_RandomMesh)))