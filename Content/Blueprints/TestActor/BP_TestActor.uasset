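; BP_TestActor is a test actor whose static mesh is set to a random mesh requested from the Game State.
; On BeginPlay it casts the Game State to BPI_GameState, caches it and calls RequestRandomMesh with itself.
; SetRandomMesh applies the supplied mesh to the StaticMesh component, and RepeatRequest asks again through the cached reference.
; ClearUP nulls that reference but is not called here, as EndPlay is empty.
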(event EventBeginPlay
  (bind _asbpi_game_state (Utilities|Casting|CastToBPI_GameState (Game|GetGameState)))
  (bind _output_get (Variables|Default|SetAs%20BPI%20Game%20State _asbpi_game_state))
  (Default|RequestRandomMesh _output_get self))

(event EventEndPlay
  (params (EndPlayReason :type EEndPlayReason%20Enum :default "Destroyed")))

(event EventRepeatRequest
  (Default|RequestRandomMesh (Variables|Default|GetAs%20BPI%20Game%20State) self))

(event EventSetRandomMesh
  (params (RandomMesh :type Static%20Mesh%20Object%20Reference))
  (Components|StaticMesh|SetStaticMesh (Variables|Default|GetStaticMesh) RandomMesh))

(fn ConstructionScript)

(fn ClearUP
  (Variables|Default|SetAs%20BPI%20Game%20State 0))