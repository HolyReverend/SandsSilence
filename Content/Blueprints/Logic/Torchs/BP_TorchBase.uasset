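; Base torch Blueprint, an interactable object whose fire effect and point light are shown or hidden through interaction.
; The construction script sets the visibility of both components from the inherited interactable status, Activated or Deactivated.
; Each interaction calls the parent handler, then a FlipFlop alternates showing and hiding them.
; The FlipFlop always shows first and does not read the status, so a torch that starts Activated stays lit on the first interaction.
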(event EventBeginInteracttoObject
  (|CallParentFunction)
  (Utilities|FlowControl|FlipFlop
    (:A
      (Rendering|SetVisibility (Variables|Default|GetPointLight) true true))
    (:B
      (Rendering|SetVisibility (Variables|Default|GetPointLight) false true))))

(fn ConstructionScript
  (|CallParentFunction)
  (switch Utilities|FlowControl|Switch|SwitchonE_InteractableStatus (CallFunction|GetInteractableStatus)
    (:NewEnumerator0
      (Rendering|SetVisibility (Variables|Default|GetPointLight) false true))
    (:NewEnumerator1
      (Rendering|SetVisibility (Variables|Default|GetPointLight) true true))))