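; Toggleable interactable that moves a scene component between two poses by hinging or sliding along a chosen axis, offset from its starting transform.
; A timeline lerps the relative transform, updates Deactivated/InProgress/Activated status, fires start and finish events, and reverses when retriggered mid-move.
; Timers add optional start and return delays, while loop modes chain finish events to cycle from BeginPlay or first interaction.
; Construction pre-poses instances set to Activated.
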(event Custom|Looping
  (Utilities|FlowControl|Delay (Variables|Settings|Timers|GetStartInteractDelayTime))
  (CallFunction|StartTimeline))

(event Custom|StartTimeline
  (switch Utilities|FlowControl|Switch|SwitchonE_InteractableStatus (CallFunction|GetInteractableStatus)
    (:NewEnumerator0
      (bind (_direction _alphavalue) (Timeline|MovingTimeline Play)
        (:Update
          (Variables|Default|SetMovingDirection _direction)
          (Variables|Default|SetMovingAlphaValue _alphavalue)
          (Transformation|SetRelativeTransform (Variables|Default|GetMovableScene) (Math|Transform|Lerp(Transform) (Variables|Default|GetStartMovableScene) (Variables|Default|GetTargetMovableScene) (Variables|Default|GetMovingAlphaValue)) false false)
          (if (not (Variables|Default|GetMovableInteractionInProgress))
            (Variables|Default|SetMovableInteractionInProgress true)
            (Variables|Default|SetInteractableStatusCash (CallFunction|GetInteractableStatus))
            (CallFunction|SetInteractableStatus "NewEnumerator2")
            (Default|CallStartMovableInteractioninProgress)))
        (:Finished
          (switch Utilities|FlowControl|Switch|SwitchonETimelineDirection (Variables|Default|GetMovingDirection)
            (:Forward
              (CallFunction|SetInteractableStatus "NewEnumerator1")
              (Variables|Default|SetMovableInteractionInProgress false)
              (if (States|IsNewInteractableStatus)
                (Default|CallFinishStartInteraction)))
            (:Backward
              (CallFunction|SetInteractableStatus "NewEnumerator0")
              (Variables|Default|SetMovableInteractionInProgress false)
              (if (States|IsNewInteractableStatus)
                (Default|CallFinishEndInteraction)))))))
    (:NewEnumerator1
      (Timeline|MovingTimeline Reverse))
    (:NewEnumerator2
      (switch Utilities|FlowControl|Switch|SwitchonETimelineDirection (Variables|Default|GetMovingDirection)
        (:Forward
          (Timeline|MovingTimeline Reverse))
        (:Backward
          (Timeline|MovingTimeline Play))))))

(event EventBeginInteracttoObject
  (switch Utilities|FlowControl|Switch|SwitchonE_LoopState (Variables|Settings|Movable|GetLoopState)
    (:NewEnumerator2
      _)
    (:NewEnumerator1
      (EventDispatchers|BindEventtoFinishStartInteraction (delegate Custom|Looping))
      (EventDispatchers|BindEventtoFinishEndInteraction (delegate Custom|Looping))))
  (if (not (Utilities|Time|IsValidTimerHandle (Variables|Handlers|GetReturnInteractDelayHandler)))
    (|CallParentFunction)
    (if (> (Variables|Settings|Timers|GetStartInteractDelayTime) 0.0)
      (Timers|StartInteractDelay)
      (else
        (CallFunction|StartTimeline)))))

(event EventBeginPlay
  (|CallParentFunction)
  (Variables|Default|SetTargetMovableScene (Moves|FindMovableSceneTransform false))
  (if (> (Variables|Settings|Timers|GetReturnInteractDelayTime) 0.0)
    (EventDispatchers|BindEventtoFinishStartInteraction (EventDispatchers|CreateEvent :!event ReturnInteractDelay)))
  (switch Utilities|FlowControl|Switch|SwitchonE_LoopState (Variables|Settings|Movable|GetLoopState)
    (:NewEnumerator0
      (EventDispatchers|BindEventtoFinishStartInteraction (delegate Custom|Looping))
      (EventDispatchers|BindEventtoFinishEndInteraction (delegate Custom|Looping))
      (CallFunction|Looping))))

(fn ConstructionScript
  (|CallParentFunction)
  (Variables|Default|SetStartMovableScene (Transformation|GetRelativeTransform (Variables|Default|GetMovableScene)))
  (CallFunction|SetPlayTimelineRate (Variables|Default|GetMovingTimeline) (Variables|Settings|Movable|GetMovingPlayRate))
  (Moves|SetMovableTypePosition))

(fn SetPlayRateMovingTimeline
  (Components|Timeline|SetPlayRate (Variables|Default|GetMovingTimeline) (/ 1.0 (Variables|Settings|Movable|GetMovingPlayRate)))
  (return))

(fn FindMovableSceneTransform
  (params (IsCounstruct :type Boolean))
  (bind _startmovablescene (Variables|Default|GetStartMovableScene))
  (bind _startmovablescene_2 (Variables|Default|GetStartMovableScene))
  (bind _startmovablescene_3 (Variables|Default|GetStartMovableScene))
  (bind _startmovablescene_4 (Variables|Default|GetStartMovableScene))
  (bind _startmovablescene_5 (Variables|Default|GetStartMovableScene))
  (bind (_roll _pitch _yaw) (Math|Rotator|BreakRotator (.rotation _startmovablescene_5)))
  (bind (_x _y _z) (Math|Vector|BreakVector (.location _startmovablescene)))
  (bind (_x_2 _y_2 _z_2) (Math|Vector|BreakVector (.location _startmovablescene_3)))
  (bind (_x_3 _y_3 _z_3) (Math|Vector|BreakVector (.location _startmovablescene_2)))
  (bind (_roll_2 _pitch_2 _yaw_2) (Math|Rotator|BreakRotator (.rotation _startmovablescene_4)))
  (return (Utilities|Select :Index (Variables|Settings|Movable|GetE_InteractableMovingType) :NewEnumerator0 (Math|Transform|MakeTransform (.location _startmovablescene_4) (Math|Rotator|MakeRotator _roll_2 _pitch_2 (States|GetValueInteractStatus _yaw_2 IsCounstruct)) (.scale _startmovablescene_4)) :NewEnumerator1 (Math|Transform|MakeTransform (.location _startmovablescene_5) (Math|Rotator|MakeRotator (States|GetValueInteractStatus _roll IsCounstruct) _pitch _yaw) (.scale _startmovablescene_5)) :NewEnumerator2 (Math|Transform|MakeTransform (Math|Vector|MakeVector (States|GetValueInteractStatus _x IsCounstruct) _y _z) (.rotation _startmovablescene) (.scale _startmovablescene)) :NewEnumerator3 (Math|Transform|MakeTransform (Math|Vector|MakeVector _x_3 (States|GetValueInteractStatus _y_3 IsCounstruct) _z_3) (.rotation _startmovablescene_2) (.scale _startmovablescene_2)) :NewEnumerator4 (Math|Transform|MakeTransform (Math|Vector|MakeVector _x_2 _y_2 (States|GetValueInteractStatus _z_2 IsCounstruct)) (.rotation _startmovablescene_3) (.scale _startmovablescene_3)))))

(fn GetValueInteractStatus
  (params (InValue :type Float%20%28double-precision%29) (IsConstruct :type Boolean))
  (return (Math|Float|SelectFloat (+ (Variables|Settings|Movable|GetMovingTargetOffset) InValue) (Math|Float|SelectFloat InValue (+ InValue (Variables|Settings|Movable|GetMovingTargetOffset)) IsConstruct) (Utilities|Enum|Equal(Enum) (CallFunction|GetInteractableStatus) "NewEnumerator1"))))

(fn SetMovableTypePosition
  (switch Utilities|FlowControl|Switch|SwitchonE_InteractableStatus (CallFunction|GetInteractableStatus)
    (:NewEnumerator0
      _)
    (:NewEnumerator1
      (Transformation|SetRelativeTransform (Variables|Default|GetMovableScene) (Moves|FindMovableSceneTransform true) false false)
      (return))
    (:NewEnumerator2
      (CallFunction|SetInteractableStatus "NewEnumerator0")))
  (return))

(fn StartInteractDelay
  (switch Utilities|FlowControl|Switch|SwitchonE_InteractableStatus (CallFunction|GetInteractableStatus)
    (:NewEnumerator0
      (if (not (Utilities|Time|IsValidTimerHandle (Variables|Handlers|GetStartInteractDelayHandler)))
        (bind _returnvalue (Utilities|Time|SetTimerbyEvent (EventDispatchers|CreateEvent :!event Custom|StartTimeline) (Variables|Settings|Timers|GetStartInteractDelayTime)))
        (Variables|Handlers|SetStartInteractDelayHandler _returnvalue)
        (EventDispatchers|BindEventtoFinishStartInteraction (EventDispatchers|CreateEvent :!event ClearStartInteractDelayHandler))
        (return)
        (else
          _)))
    (:NewEnumerator1
      (CallFunction|StartTimeline :!label _label))
    (:NewEnumerator2
      (goto _label)))
  (Handlers|ClearStartInteractDelayHandler)
  (return))

(fn ClearStartInteractDelayHandler
  (Utilities|Time|ClearandInvalidateTimerbyHandle (Variables|Handlers|GetStartInteractDelayHandler))
  (return))

(fn ClearReturnInteractDelayHandler
  (Utilities|Time|ClearandInvalidateTimerbyHandle (Variables|Handlers|GetReturnInteractDelayHandler))
  (return))

(fn CheckStartInteractDelayHandler
  (return (Utilities|Time|IsValidTimerHandle (Variables|Handlers|GetStartInteractDelayHandler))))

(fn ReturnInteractDelay
  (switch Utilities|FlowControl|Switch|SwitchonE_InteractableStatus (CallFunction|GetInteractableStatus)
    (:NewEnumerator0
      _)
    (:NewEnumerator1
      (if (not (Utilities|Time|IsValidTimerHandle (Variables|Handlers|GetReturnInteractDelayHandler)))
        (bind _returnvalue (Utilities|Time|SetTimerbyEvent (EventDispatchers|CreateEvent :!event Custom|StartTimeline) (Variables|Settings|Timers|GetReturnInteractDelayTime)))
        (Variables|Handlers|SetReturnInteractDelayHandler _returnvalue)
        (EventDispatchers|BindEventtoFinishEndInteraction (EventDispatchers|CreateEvent :!event ClearReturnInteractDelayHandler))
        (return)
        (else
          (Handlers|ClearReturnInteractDelayHandler)
          (return))))
    (:NewEnumerator2
      _))
  (return))

(fn ClearUp
  (|CallParentFunction)
  (EventDispatchers|UnbindallEventsfromFinishStartInteraction)
  (EventDispatchers|UnbindallEventsfromFinishEndInteraction)
  (Handlers|ClearStartInteractDelayHandler)
  (Handlers|ClearReturnInteractDelayHandler)
  (return))

(fn CheckReturnInteractDelayHandler
  (return (or (> (Variables|Settings|Timers|GetReturnInteractDelayTime) 0.0) (Utilities|Time|IsValidTimerHandle (Variables|Handlers|GetReturnInteractDelayHandler)))))

(fn IsNewInteractableStatus
  (return (Utilities|Enum|NotEqual(Enum) (CallFunction|GetInteractableStatus) (Variables|Default|GetInteractableStatusCash))))

(fn GetInteractableMovable
  (return self))

(fn GetReturnTotalDelayTime
  (return (+ (Variables|Settings|Timers|GetStartInteractDelayTime) (Variables|Settings|Timers|GetReturnInteractDelayTime))))