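; An interactable object that rotates its scene component in yaw by a set angle step each time the player interacts with it.
; A timeline lerps the relative rotation along the shortest path, with its play rate set from RotationTime in the construction script.
; While turning, it changes its interactable status to block re-triggering, then calls start and finish notifications.
; On finish, it recomputes the next target from the current rotation.
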(event Custom|StartRotatorTimeline
  (bind _alphavalue (Timeline|RotatorTimeline PlayFromStart)
    (:Update
      (Transformation|SetRelativeRotation (Variables|Default|GetRotationScene) (Math|Rotator|Lerp(Rotator) (Variables|Default|GetStartRotation) (Variables|Default|GetTargetRotation) _alphavalue true) false false)
      (if (not (Variables|Default|GetRotationInteractionInProgress))
        (Variables|Default|SetRotationInteractionInProgress true)
        (CallFunction|SetInteractableStatus "NewEnumerator2")
        (Default|CallStartRotationinProgress)))
    (:Finished
      (CallFunction|SetRotator)
      (CallFunction|SetInteractableStatus "NewEnumerator0")
      (Default|CallFinishEndRotation)
      (Variables|Default|SetRotationInteractionInProgress false))))

(event EventBeginPlay
  (|CallParentFunction)
  (CallFunction|SetRotator))

(event EventBeginInteracttoObject
  (if (Utilities|Enum|NotEqual(Enum) (CallFunction|GetInteractableStatus) "NewEnumerator2")
    (CallFunction|StartRotatorTimeline)))

(fn ConstructionScript
  (|CallParentFunction)
  (CallFunction|SetPlayTimelineRate (Variables|Default|GetRotatorTimeline) (Variables|Settings|Rotator|GetRotationTime)))

(fn SetRotator
  (Variables|Default|SetStartRotation (Variables|/Script/Engine.SceneComponent|GetRelativeRotation (Variables|Default|GetRotationScene)))
  (Variables|Default|SetTargetRotation (Math|Rotator|MakeRotator (.roll (Variables|Default|GetStartRotation)) (.pitch (Variables|Default|GetStartRotation)) (+ (.yaw (Variables|Default|GetStartRotation)) (Variables|Settings|Rotator|GetRotationAngle))))
  (return))

(fn ClearUp
  (Variables|Default|SetStartRotation "0, 0, 0")
  (Variables|Default|SetTargetRotation "0, 0, 0")
  (Variables|Default|SetRotationAlpha 0.0)
  (|CallParentFunction))