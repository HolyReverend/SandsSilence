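; Base Blueprint for interactable world objects that activate on overlap or on use, with stubbed hooks for children.
; A box collision registers objects with overlapping actors' BPC_InteractInstigator, tracks occupants and fires first-enter and last-exit dispatchers.
; StartInteract gates BeginInteractToObject by state, instigator type and activation mode, while a helper maps status to timeline playback.
; Only Use-type objects save state and status, with a timer restoring activated ones on load.
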(event OnComponentBeginOverlap(InteractCollision)
  (params (OverlappedComponent :type Primitive%20Component%20Object%20Reference) (OtherActor :type Actor%20Object%20Reference) (OtherComp :type Primitive%20Component%20Object%20Reference) (OtherBodyIndex :type Integer) (bFromSweep :type Boolean) (SweepResult :type Hit%20Result%20Structure%20%28by%20ref%29))
  (CallFunction|InstigatorEnter OtherActor true))

(event OnComponentEndOverlap(InteractCollision)
  (params (OverlappedComponent :type Primitive%20Component%20Object%20Reference) (OtherActor :type Actor%20Object%20Reference) (OtherComp :type Primitive%20Component%20Object%20Reference) (OtherBodyIndex :type Integer))
  (CallFunction|InstigatorEnter OtherActor false))

(event Custom|BeginInteractToObject)

(event EventBeginPlay
  (Utilities|FlowControl|Delay 1.0)
  (for _array_element (Collision|GetOverlappingActors (Variables|Default|GetInteractCollision) "BP_InteractableObjectBase_C" :!class /Script/Engine.PrimitiveComponent)
    (CallFunction|InstigatorEnter _array_element true)))

(event EventEndPlay
  (params (EndPlayReason :type EEndPlayReason%20Enum :default "Destroyed"))
  (System|ClearUp))

(event EventTick
  (params (DeltaSeconds :type Float%20%28single-precision%29)))

(fn ConstructionScript
  (Components|Box|SetBoxExtent (Variables|Default|GetInteractCollision) (Variables|Settings|General|GetInteractCollisionSize) true))

(fn InstigatorEnter
  (params (InOverlappedActor :type Actor%20Object%20Reference) (IsInstigatorEnter :type Boolean))
  (bind _returnvalue (Actor|GetComponentbyClass InOverlappedActor "/Game/Blueprints/Components/Interact/BPC_InteractInstigator.BPC_InteractInstigator_C"))
  (if IsInstigatorEnter
    (bind _success (Class|BPIInteractInstigator|AddInteractableActor(Message) _returnvalue self))
    (if _success
      (Utilities|Array|AddUnique (Variables|Default|GetOverlappedActors) InOverlappedActor)
      (if (Utilities|Array|IsNotEmpty (Variables|Default|GetOverlappedActors))
        (if (not (Variables|Default|GetIsSomyoneInCollision))
          (Variables|Default|SetIsSomyoneInCollision true)
          (Default|CallFirstAnyOverlap)
          (switch Utilities|FlowControl|Switch|SwitchonE_InteractableState (Variables|Settings|General|GetInteractableState) :!label _label
            (:NewEnumerator0
              (switch Utilities|FlowControl|Switch|SwitchonE_InteractableType (Variables|Settings|Type|GetInteractableType)
                (:NewEnumerator1
                  (bind _success_2 (CallFunction|StartInteract InOverlappedActor false))
                  (return _success_2))
                (:NewEnumerator0
                  (Default|CallInteractUseReady)
                  (return false))))
            (:NewEnumerator1
              _)
            (:NewEnumerator2
              _))
          (return false)
          (else
            (return false)))
        (else
          (return false)))
      (else
        _))
    (else
      (bind _success_3 (Class|BPIInteractInstigator|RemoveInteractableActor(Message) _returnvalue self))
      (if _success_3
        (Utilities|Array|RemoveItem (Variables|Default|GetOverlappedActors) InOverlappedActor)
        (if (Utilities|Array|IsEmpty (Variables|Default|GetOverlappedActors))
          (Variables|Default|SetIsSomyoneInCollision false)
          (Default|CallEndLastOverlap)
          (goto _label)
          (else
            (return false)))
        (else
          _))))
  (return false))

(fn CheckInteractMode
  (switch Utilities|FlowControl|Switch|SwitchonE_InteractableActivateMode (Variables|Settings|General|GetInteractableActivateMode)
    (:NewEnumerator0
      (return true))
    (:NewEnumerator1
      (switch Utilities|FlowControl|Switch|SwitchonE_InteractableType (Variables|Settings|Type|GetInteractableType)
        (:NewEnumerator1
          (return (Utilities|Array|IsNotEmpty (Variables|Default|GetOverlappedActors))))
        (:NewEnumerator0
          (return true))))
    (:NewEnumerator2
      (Variables|Settings|General|SetInteractableState "NewEnumerator2")
      (return true))))

(fn CheckCanIsInteract
  (params (InInstigator :type Actor%20Object%20Reference) (InInstigatorType :type E_InteractInstigatorType%20Enum :default "NewEnumerator0"))
  (switch Utilities|FlowControl|Switch|SwitchonE_InteractInstigatorType InInstigatorType
    (:NewEnumerator0
      (return (or (CallFunction|CheckIsPlayer InInstigator) (Utilities|DoesObjectImplementInterface InInstigator "/Game/Blueprints/Interfaces/Interact/BPI_Interactable.BPI_Interactable_C"))))
    (:NewEnumerator1
      (return (CallFunction|CheckIsPlayer InInstigator)))
    (:NewEnumerator2
      (return (and (not (CallFunction|CheckIsPlayer InInstigator)) (Utilities|DoesObjectImplementInterface InInstigator "/Game/Blueprints/Interfaces/Interact/BPI_Interactable.BPI_Interactable_C"))))))

(fn GetInteractableStatus
  (return (Variables|Settings|General|GetInteractableStatus)))

(fn SetInteractableStatus
  (params (InInteractableStatus :type E_InteractableStatus%20Enum :default "NewEnumerator0"))
  (Variables|Settings|General|SetInteractableStatus InInteractableStatus)
  (return))

(fn GetInteractableState
  (return (Variables|Settings|General|GetInteractableState)))

(fn SetInteractableState
  (params (InInteractableState :type E_InteractableState%20Enum :default "NewEnumerator0"))
  (Variables|Settings|General|SetInteractableState InInteractableState)
  (return))

(fn ClearUp
  (Utilities|Array|Clear (Variables|Default|GetOverlappedActors))
  (EventDispatchers|UnbindallEventsfromFirstAnyOverlap)
  (EventDispatchers|UnbindallEventsfromEndLastOverlap)
  (EventDispatchers|UnbindallEventsfromInteractUseReady)
  (EventDispatchers|UnbindallEventsfromBeginUse)
  (Variables|Default|SetInteractInstigator 0)
  (return))

(fn GetInteractableType
  (return (Variables|Settings|Type|GetInteractableType)))

(fn GetSomyoneinCollision
  (return (Variables|Default|GetIsSomyoneInCollision)))

(fn GetInteractableTimeline
  (params (InTimelineDirection :type ETimelineDirection%20Enum%20%28by%20ref%29 :default "Forward"))
  (switch Utilities|FlowControl|Switch|SwitchonE_InteractableStatus (Variables|Settings|General|GetInteractableStatus)
    (:NewEnumerator0
      (bind _output_get (Variables|States|SetInteractableTimeline "NewEnumerator1")))
    (:NewEnumerator1
      (bind _output_get_2 (Variables|States|SetInteractableTimeline "NewEnumerator4")))
    (:NewEnumerator2
      (switch Utilities|FlowControl|Switch|SwitchonETimelineDirection InTimelineDirection
        (:Forward
          (bind _output_get_3 (Variables|States|SetInteractableTimeline "NewEnumerator3")))
        (:Backward
          (bind _output_get_4 (Variables|States|SetInteractableTimeline "NewEnumerator0"))))))
  (return (Utilities|Select :Index (Variables|States|GetInteractableTimeline) :NewEnumerator0 _output_get_4 :NewEnumerator1 _output_get :NewEnumerator2 "NewEnumerator2" :NewEnumerator3 _output_get_3 :NewEnumerator4 _output_get_2 :NewEnumerator5 "NewEnumerator5")))

(fn GetInteractInstigator
  (return (Variables|Default|GetInteractInstigator)))

(fn LoadData)

(fn CheckReturnInteractDelayHandler
  (return false))

(fn CheckStartInteractDelayHandler)

(fn GetInteractableMovable
  (return 0))

(fn GetInteractableObject
  (return self))

(fn GetLocationSaveData
  (return false "0, 0, 0"))

(fn GetLogicSaveData
  (if (Utilities|Enum|Equal(Enum) (States|GetInteractableType) "NewEnumerator0")
    (return true (Utilities|Struct|MakeST_LogicObjectSaveData (States|GetInteractableState) (States|GetInteractableStatus)))
    (else
      (return false ""))))

(fn GetReturnTotalDelayTime
  (return 0.0))

(fn GetRotationSaveData
  (return false "0, 0, 0"))

(fn SetLocationLoadData
  (params (InLocation :type Vector :default "0, 0, 0"))
  (return false))

(fn SetLogicLoadData
  (params (InLogic :type ST%20Logic%20Object%20Save%20Data%20Structure))
  (if (Utilities|Enum|Equal(Enum) (States|GetInteractableType) "NewEnumerator0")
    (if (Utilities|Enum|Equal(Enum) (Utilities|Struct|BreakST_LogicObjectSaveData InLogic) "NewEnumerator1")
      (Utilities|Time|SetTimerbyEvent (EventDispatchers|CreateEvent :!event Custom|BeginInteractToObject) (Variables|/Game/Data/DataAssets/System/BPDA_GlobalSettings.BPDA_GlobalSettings_C|GetLogicLoadTimeStart (Variables|System|GetGlobalSettings)))
      (return true)
      (else
        (return false)))
    (else
      (return false))))

(fn SetRotationLoadData
  (params (InRotation :type Rotator :default "0, 0, 0"))
  (return false))

(fn StartInteract
  (params (InInstigator :type Actor%20Object%20Reference%20%28by%20ref%29) (IsActionUse :type Boolean))
  (switch Utilities|FlowControl|Switch|SwitchonE_InteractableState (Variables|Settings|General|GetInteractableState)
    (:NewEnumerator0
      (if (States|CheckCanIsInteract InInstigator (Variables|Settings|Type|GetInstigatorType))
        _
        (else
          (return false))))
    (:NewEnumerator1
      (if (States|CheckCanIsInteract InInstigator "NewEnumerator2")
        _
        (else
          (return false))))
    (:NewEnumerator2
      (return false)))
  (if (States|CheckInteractMode)
    (if (not IsActionUse)
      _
      (elif (Utilities|Enum|Equal(Enum) (Variables|Settings|Type|GetInteractableType) "NewEnumerator0")
        (Variables|Default|SetInteractInstigator InInstigator)
        (else
          (return false))))
    (CallFunction|BeginInteracttoObject)
    (return true)
    (else
      (return false))))