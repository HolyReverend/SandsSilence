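; Base Blueprint for a beam mechanism that shows a Niagara beam and spotlight, aimed at mirror mechanism locations.
; It builds a beam ray struct from its arrow and rotated mesh at construction and BeginPlay, exposed through getters.
; Interaction uses parent behavior when IsRotation is valid, otherwise an empty TryInteractToBeam event.
; Events switch the effects on, off or off after a timer; distance-based material intensity logic is disconnected.
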(event Custom|TryInteractToBeam)

(event EventBeginPlay
  (|CallParentFunction)
  (CallFunction|SetBeamRay)
  (bind _returnvalue (Rendering|Material|CreateDynamicMaterialInstance (Variables|Default|GetRotatedMesh) 0 "/Game/LevelPrototyping/Blocking/Materials/Instances/StylizedEgypt/MI_part_ornament_01_Inst.MI_part_ornament_01_Inst" "None" :!class /Script/Engine.PrimitiveComponent))
  (Variables|Default|SetDynamicMaterial _returnvalue))

(event EventBeamEnable
  (params (InCurrentMirrorMechLocation :type Vector%20%28by%20ref%29 :default "0, 0, 0"))
  (Effects|Components|ParticleSystem|SetVectorParameter (Variables|Default|GetNS_Beam) "Beam End" InCurrentMirrorMechLocation)
  (Components|Activation|Activate (Variables|Default|GetNS_Beam) false)
  (Rendering|SetVisibility (Variables|Default|GetSpotLight) true true))

(event EventBeamDisable
  (Components|Activation|Deactivate (Variables|Default|GetNS_Beam))
  (Rendering|SetVisibility (Variables|Default|GetSpotLight) false true))

(event EventBeginInteracttoObject
  (Variables|Settings|Beam|GetIsRotation
    (:then
      (|CallParentFunction))
    (:else
      (CallFunction|TryInteracttoBeam))))

(event EventDelayBeamDisable
  (params (InTimeDelay :type Float%20%28double-precision%29%20%28by%20ref%29))
  (Utilities|Time|SetTimerbyEvent (delegate EventBeamDisable) InTimeDelay))

(event EventTick
  (params (DeltaSeconds :type Float%20%28single-precision%29))
  (|CallParentFunction DeltaSeconds))

(fn ConstructionScript
  (|CallParentFunction)
  (CallFunction|SetBeamRay))

(fn SetBeamRay
  (bind _beamarrow (Variables|Default|GetBeamArrow))
  (bind _rotatedmesh (Variables|Default|GetRotatedMesh))
  (Utilities|Struct|SetmembersinST_BeamRay (Variables|Default|GetBeamRay) (Transformation|GetWorldLocation _beamarrow) (Math|Vector|GetForwardVector _beamarrow) (Variables|Settings|Beam|GetBeamMaxDistance) (* (.Max (Components|StaticMesh|GetLocalBounds _rotatedmesh)) (Variables|Settings|Beam|GetWidthSizeMod)) (Transformation|GetWorldRotation _rotatedmesh))
  (return))

(fn GetBeamArrowLocation
  (return (Transformation|GetWorldLocation (Variables|Default|GetBeamArrow))))

(fn GetBeamRay
  (return (Variables|Default|GetBeamRay)))