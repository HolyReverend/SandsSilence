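; Beam puzzle emitter that traces a beam through its assigned mirrors toward a receiver.
; Interaction requests a rebuild, which box-traces from each element via BPI_Beam, using distance-over-speed timers to pace hops to the next mirror.
; Reaching the receiver changes the interactable state of emitter and mirrors and activates the receiver.
; A miss or revisited mirror schedules beam shutdown in reverse order with accumulated delays.
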(event Custom|StartBeamNetworkBuild
  (CallFunction|BuildBeamNetwork self))

(event EventBeginPlay
  (|CallParentFunction)
  (if (Utilities|Array|IsNotEmpty (Variables|Settings|Beam|GetBeamMirrors))
    (EventDispatchers|AssignBeamNetworkNeedRebuild (delegate Custom|StartBeamNetworkBuild))))

(event EventTryInteracttoBeam
  (|CallParentFunction)
  (Variables|Default|GetBeamNetworkIsBusy
    (:then)
    (:else
      (Default|CallBeamNetworkNeedRebuild))))

(fn ConstructionScript
  (|CallParentFunction))

(fn BuildBeamNetwork
  (params (InCurrentBeam :type Actor%20Object%20Reference%20%28by%20ref%29))
  (Variables|Default|SetBeamNetworkIsBusy true)
  (bind _returnvalue (Class|BPIBeam|GetBeamRay(Message) InCurrentBeam))
  (bind (_outhit _returnvalue_2) (Collision|BoxTraceByChannel (.Start (Utilities|Struct|BreakST_BeamRay _returnvalue)) (+ (.Start (Utilities|Struct|BreakST_BeamRay _returnvalue)) (* (.Direction (Utilities|Struct|BreakST_BeamRay _returnvalue)) (.MaxDistance (Utilities|Struct|BreakST_BeamRay _returnvalue)))) (.SizeModifier (Utilities|Struct|BreakST_BeamRay _returnvalue)) (.Rotation (Utilities|Struct|BreakST_BeamRay _returnvalue)) "TraceTypeQuery4" false (Utilities|Array|MakeArray InCurrentBeam) "None" true "(R=0.095695,G=0.000000,B=1.000000,A=1.000000)" "(R=1.000000,G=0.103386,B=0.000000,A=1.000000)"))
  (if _returnvalue_2
    (if (Utilities|DoesObjectImplementInterface (.HitActor (Collision|BreakHitResult _outhit)) "/Game/Blueprints/Interfaces/BPI_Beam.BPI_Beam_C")
      (bind _output_get (LocalVariables|SetL_FindedBeamMech (.HitActor (Collision|BreakHitResult _outhit))))
      (if (not (Utilities|Map|Contains (Variables|Default|GetUsedBeamMechs) _output_get))
        (LocalVariables|SetL_FindedBeamMechDistance (.Distance (Collision|BreakHitResult _outhit)))
        (bind _returnvalue_3 (Class|BPIBeam|GetBeamArrowLocation(Message) (LocalVariables|GetL_FindedBeamMech)))
        (Class|BPIBeam|BeamEnable(Message) InCurrentBeam _returnvalue_3)
        (if (== (LocalVariables|GetL_FindedBeamMech) (Variables|Settings|Beam|GetBeamReceiver))
          (CallFunction|SuccesCreateMirrorNetwork)
          (return)
          (else
            (bind _array_element (Utilities|Array|ForEachLoopwithBreak (Variables|Settings|Beam|GetBeamMirrors) :!label _label)
              (:LoopBody
                (if (== _array_element (LocalVariables|GetL_FindedBeamMech))
                  (Utilities|Map|Add (Variables|Default|GetUsedBeamMechs) (LocalVariables|GetL_FindedBeamMech) (/ (LocalVariables|GetL_FindedBeamMechDistance) (Variables|Settings|Beam|GetBeamSpeed)))
                  (LocalVariables|SetL_BeamMechFinded true)
                  (goto _label Break)))
              (:Completed
                (LocalVariables|GetL_BeamMechFinded
                  (:then
                    (Variables|Default|SetNextBeamMirror (LocalVariables|GetL_FindedBeamMech))
                    (Utilities|Time|SetTimerbyEvent (EventDispatchers|CreateEvent :!event NextMirrorFounded) (.Value (Utilities|Map|Find (Variables|Default|GetUsedBeamMechs) (LocalVariables|GetL_FindedBeamMech))))
                    (return))
                  (:else
                    (CallFunction|ClearMirrorNetwork)
                    (return)))))))
        (else
          (CallFunction|BeamsDisable :!label _label_2)
          (return)))
      (else
        (Class|BPIBeam|BeamEnable(Message) InCurrentBeam (.TraceEnd (Collision|BreakHitResult _outhit)) :!label _label_3)
        (goto _label_2)))
    (else
      (goto _label_3))))

(fn ClearMirrorNetwork
  (Variables|Default|SetBeamNetworkIsBusy false)
  (Variables|Default|SetNextBeamMirror 0)
  (Utilities|Map|Clear (Variables|Default|GetUsedBeamMechs))
  (return))

(fn SuccesCreateMirrorNetwork
  (for _array_element (Variables|Settings|Beam|GetBeamMirrors)
    (Default|SetInteractableState _array_element "NewEnumerator2"))
  (Default|SetInteractableState self "NewEnumerator2")
  (Default|CallBeamNetworkActivate (Variables|Settings|Beam|GetBeamReceiver))
  (CallFunction|ClearMirrorNetwork)
  (return))

(fn NextMirrorFounded
  (CallFunction|BuildBeamNetwork (Variables|Default|GetNextBeamMirror))
  (return))

(fn BeamsDisable
  (bind _keys (Utilities|Map|Keys (Variables|Default|GetUsedBeamMechs)))
  (bind _output_get (LocalVariables|SetL_ReversedUsedBeamMechs _keys))
  (Utilities|Array|Reverse _output_get)
  (for (_array_element _array_index) (LocalVariables|GetL_ReversedUsedBeamMechs)
    (LocalVariables|SetL_CurrentBeamMech _array_element)
    (LocalVariables|SetL_TimeDelayToNextBeamMech (select (== _array_index 0) (.Value (Utilities|Map|Find (Variables|Default|GetUsedBeamMechs) (LocalVariables|GetL_CurrentBeamMech))) (+ (LocalVariables|GetL_TimeDelayToNextBeamMech) (.Value (Utilities|Map|Find (Variables|Default|GetUsedBeamMechs) (LocalVariables|GetL_CurrentBeamMech))))))
    (Class|BPIBeam|DelayBeamDisable(Message) (LocalVariables|GetL_CurrentBeamMech) (LocalVariables|GetL_TimeDelayToNextBeamMech)))
  (CallFunction|DelayBeamDisable (+ (LocalVariables|GetL_TimeDelayToNextBeamMech) 0.25))
  (CallFunction|ClearMirrorNetwork)
  (return))