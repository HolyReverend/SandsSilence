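; Interactable spinner, built on a parent interactable, that ramps a RotatingMovement component between rest and a target rotation rate.
; Interaction plays, stops or reverses SpinnerTimeline according to its direction, and the timeline lerps the rate while updating status and firing in-progress, activated and deactivated calls.
; Sphere overlaps register instigators, construction sets the timeline play rate, and Tick keeps InteractCollision deactivated.
; A separate custom event eases the root's relative rotation back to zero.
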(event OnComponentBeginOverlap(SphereCollision)
  (params (OverlappedComponent :type Primitive%20Component%20Object%20Reference) (OtherActor :type Actor%20Object%20Reference) (OtherComp :type Primitive%20Component%20Object%20Reference) (OtherBodyIndex :type Integer) (bFromSweep :type Boolean) (SweepResult :type Hit%20Result%20Structure%20%28by%20ref%29))
  (CallFunction|InstigatorEnter OtherActor true))

(event OnComponentEndOverlap(SphereCollision)
  (params (OverlappedComponent :type Primitive%20Component%20Object%20Reference) (OtherActor :type Actor%20Object%20Reference) (OtherComp :type Primitive%20Component%20Object%20Reference) (OtherBodyIndex :type Integer))
  (CallFunction|InstigatorEnter OtherActor false))

(event Custom|StartTimeline
  (bind _rotatingmovement (Variables|Default|GetRotatingMovement))
  (switch Utilities|FlowControl|Switch|SwitchonE_InteractableTimeline (CallFunction|GetInteractableTimeline (Variables|System|GetMovingDirection))
    (:NewEnumerator0
      (Components|Activation|Activate _rotatingmovement false)
      (bind (_direction _alphavalue) (Timeline|SpinnerTimeline Play)
        (:Update
          (Variables|System|SetMovingDirection _direction)
          (Variables|/Script/Engine.RotatingMovementComponent|SetRotationRate (Variables|Default|GetRotatingMovement) (Math|Rotator|Lerp(Rotator) (Variables|System|GetStartingRotationRate) (Variables|System|GetTargetRotationRate) _alphavalue))
          (Variables|System|GetisSpinnerInProgress
            (:then)
            (:else
              (Variables|System|SetisSpinnerInProgress true)
              (CallFunction|SetInteractableStatus "NewEnumerator2")
              (Default|CallSpinnerinProgress))))
        (:Finished
          (switch Utilities|FlowControl|Switch|SwitchonETimelineDirection (Variables|System|GetMovingDirection)
            (:Forward
              (CallFunction|SetInteractableStatus "NewEnumerator1")
              (Default|CallSpinnerActivated)
              (Variables|System|SetisSpinnerInProgress false))
            (:Backward
              (CallFunction|SetInteractableStatus "NewEnumerator0")
              (Components|Activation|Deactivate (Variables|Default|GetRotatingMovement))
              (Default|CallSpinnerDeactivated)
              (Variables|System|SetisSpinnerInProgress false))))))
    (:NewEnumerator1
      (Components|Activation|Activate _rotatingmovement false)
      (Timeline|SpinnerTimeline PlayFromStart))
    (:NewEnumerator2
      (Timeline|SpinnerTimeline Stop))
    (:NewEnumerator3
      (Timeline|SpinnerTimeline Reverse))
    (:NewEnumerator4
      (Timeline|SpinnerTimeline ReverseFromEnd))))

(event Custom|CustomEvent
  (Variables|Default|SetRelative%20Rotation (Variables|/Script/Engine.SceneComponent|GetRelativeRotation (Variables|Default|GetDefaultSceneRoot)))
  (bind _updatealpha (Timeline|Timeline Play)
    (:Update
      (Transformation|SetRelativeRotation (Variables|Default|GetDefaultSceneRoot) (Math|Rotator|Lerp(Rotator) (Variables|Default|GetRelative%20Rotation) "0, 0, 0" _updatealpha) false false))))

(event EventBeginPlay
  (|CallParentFunction)
  (Variables|System|SetStartingRotationRate "0, 0, 0")
  (Variables|System|SetTargetRotationRate (Variables|Settings|Spinner|GetSpinnerRotationRate))
  (switch Utilities|FlowControl|Switch|SwitchonE_InteractableStatus (CallFunction|GetInteractableStatus)
    (:NewEnumerator0
      (Variables|/Script/Engine.RotatingMovementComponent|SetRotationRate (Variables|Default|GetRotatingMovement) (Variables|System|GetStartingRotationRate)))
    (:NewEnumerator1
      (Variables|/Script/Engine.RotatingMovementComponent|SetRotationRate (Variables|Default|GetRotatingMovement) (Variables|System|GetTargetRotationRate)))))

(event EventTick
  (params (DeltaSeconds :type Float%20%28single-precision%29))
  (|CallParentFunction DeltaSeconds)
  (Components|Activation|Deactivate (Variables|Default|GetInteractCollision)))

(event EventBeginInteracttoObject
  (CallFunction|StartTimeline))

(fn ConstructionScript
  (|CallParentFunction)
  (CallFunction|SetPlayTimelineRate (Variables|Default|GetSpinnerTimeline) (Variables|Settings|Spinner|GetMovingPlayRate)))