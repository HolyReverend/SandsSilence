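; Base Blueprint for pushable objects that the player attaches to and releases through interaction.
; On interact, it checks that the instigator is the player, then messages that character's push component to begin or end pushing, passing attach points and attach duration.
; The construction script adds an arrow component at each attach point transform.
; Save functions expose the root's world location and restore it by teleporting on load.
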(event Custom|TryPushing
  (if (== (CallFunction|GetInteractInstigator) (CallFunction|GetActualPlayer))
    (bind _returnvalue (Class|BPIPlayerCharacter|GetPushComponent(Message) (CallFunction|GetInteractInstigator)))
    (bind _isvalid (Class|BPIPush|CheckCharactaerIsPushing(Message) _returnvalue))
    (if (not _isvalid)
      (Class|BPIPush|BeginPushing(Message) _returnvalue self (Variables|Settings|Move|GetPushAttachPoint) (Variables|Settings|Move|GetTimeAttachDuration))
      (else
        (Class|BPIPush|EndPushing(Message) _returnvalue self)))))

(event EventBeginPlay
  (|CallParentFunction))

(event EventBeginInteracttoMovableObject
  (|CallParentFunction)
  (CallFunction|TryPushing))

(fn ConstructionScript
  (|CallParentFunction)
  (for _array_element (Variables|Settings|Move|GetPushAttachPoint)
    (AddComponent|AddArrowComponent false _array_element)))

(fn GetLocationSaveData
  (return true (Transformation|GetWorldLocation (Variables|Default|GetDefaultSceneRoot))))

(fn SetLocationLoadData
  (params (InLocation :type Vector :default "0, 0, 0"))
  (Transformation|SetWorldLocation (Variables|Default|GetDefaultSceneRoot) InLocation false true)
  (return true))