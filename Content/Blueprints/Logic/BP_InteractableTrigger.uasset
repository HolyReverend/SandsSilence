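; Interactable trigger, such as a switch, that forwards its interaction to a list of TriggeredObjects, with optional movement of its own.
; It fires them on interaction begin when set to run immediately, otherwise binds to its own start/end finish events and changes state while triggering.
; It tracks the triggered actor with the longest return delay and binds to its end event, otherwise resetting its interactable state directly.
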(event Custom|ReturnTriggerAfterCompletetInteract
  (CallFunction|StartTimeline)
  (EventDispatchers|UnbindallEventsfromFinishEndInteraction)
  (EventDispatchers|AssignFinishEndInteraction (delegate Custom|ReturnEnableState)))

(event Custom|ReturnEnableState
  (CallFunction|SetInteractableState "NewEnumerator0")
  (EventDispatchers|UnbindallEventsfromFinishEndInteraction))

(event EventBeginPlay
  (Variables|Settings|Trigger|GetIsMovable
    (:then
      (|CallParentFunction))
    (:else
      _))
  (if (not (Variables|Settings|Trigger|GetisRunTriggerImmediately))
    (EventDispatchers|BindEventtoFinishStartInteraction (EventDispatchers|CreateEvent :!event SendtoTriggeredInteraction))
    (EventDispatchers|BindEventtoFinishEndInteraction (EventDispatchers|CreateEvent :!event SendtoTriggeredInteraction))))

(event EventTick
  (params (DeltaSeconds :type Float%20%28single-precision%29))
  (|CallParentFunction DeltaSeconds))

(event EventBeginInteracttoObject
  (Variables|Settings|Trigger|GetIsMovable
    (:then
      (|CallParentFunction))
    (:else
      _))
  (Variables|Settings|Trigger|GetisRunTriggerImmediately
    (:then
      (Interaction|SendtoTriggeredInteraction))
    (:else)))

(fn ConstructionScript
  (|CallParentFunction))

(fn SendtoTriggeredInteraction
  (if (Utilities|Array|IsNotEmpty (Variables|Settings|Trigger|GetTriggeredObjects))
    (if (not (Variables|Settings|Trigger|GetisRunTriggerImmediately))
      (CallFunction|SetInteractableState "NewEnumerator2"))
    (for _array_element (Variables|Settings|Trigger|GetTriggeredObjects)
      (bind _output_get (LocalVariables|SetL_CurrentTriggeredActor _array_element))
      (Default|StartInteract _output_get self false)
      (bind _isvalide (Default|CheckReturnInteractDelayHandler (LocalVariables|GetL_CurrentTriggeredActor)))
      (if _isvalide
        (LocalVariables|SetL_IsReturnInteractDelayValid true)
        (bind _returnvalue (Default|GetReturnTotalDelayTime (LocalVariables|GetL_CurrentTriggeredActor)))
        (Utilities|IsValid (LocalVariables|GetL_MostTotalTimeTriggeredActor)
          (:Is%20Valid
            (bind _returnvalue_2 (Default|GetReturnTotalDelayTime (LocalVariables|GetL_MostTotalTimeTriggeredActor)))
            (if (< _returnvalue_2 _returnvalue)
              (LocalVariables|SetL_MostTotalTimeTriggeredActor (LocalVariables|GetL_CurrentTriggeredActor))))
          (:Is%20Not%20Valid
            (LocalVariables|SetL_MostTotalTimeTriggeredActor (LocalVariables|GetL_CurrentTriggeredActor))))
        (else
          (LocalVariables|SetL_MostTotalTimeTriggeredActor (LocalVariables|GetL_CurrentTriggeredActor)))))
    (LocalVariables|GetL_IsReturnInteractDelayValid
      (:then
        (bind _returnvalue_3 (Default|GetInteractableMovable (LocalVariables|GetL_MostTotalTimeTriggeredActor)))
        (EventDispatchers|BindEventtoFinishEndInteraction _returnvalue_3 (EventDispatchers|CreateEvent :!event Custom|ReturnTriggerAfterCompletetInteract))
        (return))
      (:else
        (if (Variables|Settings|Trigger|GetisRunTriggerImmediately)
          (CallFunction|StartTimeline)
          (CallFunction|SetInteractableState "NewEnumerator0")
          (else
            (CallFunction|SetInteractableState "NewEnumerator0")))))
    (else
      (return))))