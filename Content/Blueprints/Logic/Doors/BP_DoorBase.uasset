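; BP_DoorBase is a base door Blueprint whose BeginPlay and construction script only call their parents.
; It defines events that turn DoorMesh collision off and restore it from DoorCollisionPreset.
; Logic to cache that collision setting and bind these events to interaction start and finish delegates, disabling collision during movement, is present but unconnected, so it never runs.
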(event Custom|EnableDoorCollision
  (Collision|SetCollisionEnabled (Variables|Default|GetDoorMesh) (Variables|Default|GetDoorCollisionPreset)))

(event Custom|DisableDoorCollision
  (Collision|SetCollisionEnabled (Variables|Default|GetDoorMesh) "NoCollision"))

(event EventBeginPlay
  (|CallParentFunction))

(fn ConstructionScript
  (|CallParentFunction))