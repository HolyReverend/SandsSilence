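; Anim notify state that triggers climb IK for reaching a ledge in the parkour system.
; The begin event does nothing; on end it calls the parent, then acts only when SecondIK is set.
; It then tells the owner's BPC_Parkour component to compute hand and foot placement via StartClimbIKMessage, passing InFirst as false and the side from WhichHand.
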(fn ReceivedNotifyBegin
  (params (MeshComp :type Skeletal%20Mesh%20Component%20Object%20Reference) (Animation :type Anim%20Sequence%20Base%20Object%20Reference) (TotalDuration :type Float%20%28single-precision%29) (EventReference :type Anim%20Notify%20Event%20Reference%20Structure%20%28by%20ref%29))
  (return false))

(fn ReceivedNotifyEnd
  (params (MeshComp :type Skeletal%20Mesh%20Component%20Object%20Reference) (Animation :type Anim%20Sequence%20Base%20Object%20Reference) (EventReference :type Anim%20Notify%20Event%20Reference%20Structure%20%28by%20ref%29))
  (|CallParentFunction MeshComp Animation EventReference)
  ;[0.15 0.15 0.15 0.5] Посылаем в BPC_Parkour команду, что необходимо посчитать где должны находиться руки и ноги
  (if (Variables|Default|GetSecondIK)
    (bind _success (Class|BPIParkourLogic|StartClimbIK(Message) (Actor|GetComponentbyClass (Components|GetOwner MeshComp) "/Game/Blueprints/Components/Character/BPC_Parkour.BPC_Parkour_C") (not (Variables|Default|GetSecondIK)) (== (Variables|Default|GetWhichHand) "(TagName=\"Parkour.Direction.Right\")")))
    (return _success)
    (else
      (return false))))